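; BP_EnemySpawner is a test spawner for trying out spawn locations, but as wired it spawns nothing.
; BeginPlay starts a looping timer on SpawnProjectile, which has an empty body.
; Disconnected logic would spawn a BP_PaperProjectile at one of three scene component locations chosen at random.
; A random pick from an EnemiesToSpawn array is also left unused.
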(event `self.ReceiveBeginPlay`
  ;[1 0.3216 0.1208] Testing Spawn Locations
  (`KismetSystemLibrary.K2_SetTimerDelegate` (delegate `SpawnProjectile`) 1.0 true))

(event `SpawnProjectile`)

(fn `UserConstructionScript`)