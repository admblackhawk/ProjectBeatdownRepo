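; BP_PouchProjectile is a pouch projectile that explodes on characters' capsules unless it has been deflected.
; It plays a swoosh on spawn, and overlapping any capsule component triggers a wrong-note sound, impact sound and explosion emitter, then destroys the actor.
; The PouchDeflected event sets a flag that disables that hit response, plays a note and impact sound, and tints the pouch light blue through a dynamic material instance.
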(event `self.ReceiveBeginPlay`
  (`GameplayStatics.PlaySoundAtLocation` "/Game/_Main/Music/heavy_swosh_effect.heavy_swosh_effect" (`SceneComponent.K2_GetComponentLocation` (`self.PouchMesh`)) (struct) 1.0 1.0 0.0 null null null null))

(event `PouchDeflected`
  (bind _returnvalue (`SceneComponent.K2_GetComponentLocation` (`self.PouchMesh`)))
  (set `self.IsPouchDeflected?` true)
  (`GameplayStatics.PlaySoundAtLocation` "/Game/_Main/Music/note4.note4" _returnvalue (struct) 1.0 1.0 0.0 null null null null)
  (`GameplayStatics.PlaySoundAtLocation` "/Game/_Main/Music/pouch_impact_only.pouch_impact_only" _returnvalue (struct) 1.0 1.0 0.0 null null null null)
  (bind _returnvalue_2 (`PrimitiveComponent.CreateDynamicMaterialInstance` (`self.PouchMesh`) 0 "/Game/_Main/Blueprints/MT_PouchMat.MT_PouchMat" "None"))
  (`MaterialInstanceDynamic.SetVectorParameterValue` _returnvalue_2 "PouchColor" (struct :`R` 0.489158 :`G` 0.666189 :`B` 1.0 :`A` 1.0)))

(event `self.PouchMesh.OnComponentBeginOverlap`
  (params (OverlappedComponent :type "PrimitiveComponent Object Reference") (OtherActor :type "Actor Object Reference") (OtherComp :type "PrimitiveComponent Object Reference") (OtherBodyIndex :type Integer) (bFromSweep :type Boolean) (SweepResult :type "HitResult Structure (by ref)"))
  (bind _returnvalue (`SceneComponent.K2_GetComponentLocation` (`self.PouchMesh`)))
  (if (not (`self.IsPouchDeflected?`))
    (cast `CapsuleComponent` OtherComp)
    (`GameplayStatics.PlaySoundAtLocation` "/Game/_Main/Music/wrongNOTE.wrongNOTE" _returnvalue (struct) 1.0 1.0 0.0 null null null null)
    (`GameplayStatics.PlaySoundAtLocation` "/Game/_Main/Music/pouch_impact.pouch_impact" _returnvalue (struct) 1.0 1.0 0.0 null null null null)
    (`GameplayStatics.SpawnEmitterAtLocation` "/Game/StarterContent/Particles/P_Explosion.P_Explosion" _returnvalue)
    (`self.K2_DestroyActor`)))

(fn `UserConstructionScript`)