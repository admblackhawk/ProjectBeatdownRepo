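; BP_PaperProjectile is a paper projectile that explodes on overlapping a capsule component unless it has been deflected.
; It plays a sound on spawn, and an undeflected hit plays a failure sound, spawns an explosion emitter and destroys the actor.
; The PaperDeflected event plays a shutter sound, tints the mesh green through a dynamic material instance and sets the flag that disables the overlap response.
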(event `self.ReceiveBeginPlay`
  (`GameplayStatics.PlaySoundAtLocation` "/Engine/EditorSounds/Notifications/CompileSuccess_Cue.CompileSuccess_Cue" (`SceneComponent.K2_GetComponentLocation` (`self.PaperMesh`)) (struct) 1.0 1.0 0.0 null null null null))

(event `PaperDeflected`
  (`GameplayStatics.PlaySoundAtLocation` "/Engine/VREditor/Sounds/UI/Camera_Shutter.Camera_Shutter" (`SceneComponent.K2_GetComponentLocation` (`self.PaperMesh`)) (struct) 1.0 1.0 0.0 null null null null)
  (bind _returnvalue (`PrimitiveComponent.CreateDynamicMaterialInstance` (`self.PaperMesh`) 0 "/Game/_Main/Blueprints/MT_PaperMat.MT_PaperMat" "None"))
  (`MaterialInstanceDynamic.SetVectorParameterValue` _returnvalue "PaperColor" (struct :`R` 0.245097 :`G` 1.0 :`B` 0.363374 :`A` 1.0))
  (set `self.IsPaperDeflected?` true))

(event `self.PaperMesh.OnComponentBeginOverlap`
  (params (OverlappedComponent :type "PrimitiveComponent Object Reference") (OtherActor :type "Actor Object Reference") (OtherComp :type "PrimitiveComponent Object Reference") (OtherBodyIndex :type Integer) (bFromSweep :type Boolean) (SweepResult :type "HitResult Structure (by ref)"))
  (if (not (`self.IsPaperDeflected?`))
    (cast `CapsuleComponent` OtherComp)
    (`GameplayStatics.PlaySoundAtLocation` "/Engine/EditorSounds/Notifications/CompileFailed.CompileFailed" (`self.K2_GetActorLocation`) (struct) 1.0 1.0 0.0 null null null null)
    (`GameplayStatics.SpawnEmitterAtLocation` "/Game/StarterContent/Particles/P_Explosion.P_Explosion" (`SceneComponent.K2_GetComponentLocation` (`self.PaperMesh`)))
    (`self.K2_DestroyActor`)))

(fn `UserConstructionScript`)