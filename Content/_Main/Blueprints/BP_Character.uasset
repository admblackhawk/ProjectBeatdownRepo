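; Player character that parries paper and pouch projectiles with two separate deflect inputs.
; Each press opens a parry window that closes on release or after a short delay.
; During it, the matching collider flings overlapping projectiles back faster by negatively scaling velocity and notifies them.
; Deflect and idle animations are forwarded to BP_2dChar via GetActorOfClass, while the mesh plays simple one-shot animations; several unconnected test nodes remain.
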(event `self.ReceiveBeginPlay`
  (`SkeletalMeshComponent.PlayAnimation` (`self.Mesh`) "/Game/Characters/Mannequins/Animations/Manny/MM_Idle.MM_Idle" false))

(event `Key|W`
  (params (Key :type "Key Structure")))

(event `Key|S`
  (params (Key :type "Key Structure")))

(event `Key|A`
  (params (Key :type "Key Structure")))

(event `Key|D`
  (params (Key :type "Key Structure")))

(event `self.PaperParryCollider.OnComponentBeginOverlap`
  (params (OverlappedComponent :type "PrimitiveComponent Object Reference") (OtherActor :type "Actor Object Reference") (OtherComp :type "PrimitiveComponent Object Reference") (OtherBodyIndex :type Integer) (bFromSweep :type Boolean) (SweepResult :type "HitResult Structure (by ref)"))
  (if (`self.DeflectPaper`)
    (bind _asbp_paper_projectile (cast `/Game/_Main/Blueprints/BP_PaperProjectile` OtherActor))
    (bind _projectilemovement (`/Game/_Main/Blueprints/BP_PaperProjectile.ProjectileMovement` _asbp_paper_projectile))
    (set `MovementComponent.Velocity` (* (`MovementComponent.Velocity` _projectilemovement) -10.0) _projectilemovement)
    (`/Game/_Main/Blueprints/BP_PaperProjectile.PaperDeflected` _asbp_paper_projectile)))

(event `self.PouchParryCollider.OnComponentBeginOverlap`
  (params (OverlappedComponent :type "PrimitiveComponent Object Reference") (OtherActor :type "Actor Object Reference") (OtherComp :type "PrimitiveComponent Object Reference") (OtherBodyIndex :type Integer) (bFromSweep :type Boolean) (SweepResult :type "HitResult Structure (by ref)"))
  (if (`self.DeflectPouch`)
    (bind _asbp_pouch_projectile (cast `/Game/_Main/Blueprints/BP_PouchProjectile` OtherActor))
    (bind _pouchprojectilemovement (`/Game/_Main/Blueprints/BP_PouchProjectile.PouchProjectileMovement` _asbp_pouch_projectile))
    (set `MovementComponent.Velocity` (* (`MovementComponent.Velocity` _pouchprojectilemovement) -10.0) _pouchprojectilemovement)
    (`/Game/_Main/Blueprints/BP_PouchProjectile.PouchDeflected` _asbp_pouch_projectile)))

(event `AnimDeflectPaper`
  (bind _returnvalue (`GameplayStatics.GetActorOfClass` "/Game/_Main/Blueprints/BP_2dChar.BP_2dChar_C"))
  (`/Game/_Main/Blueprints/BP_2dChar.2dAnimCharDeflectPaper` _returnvalue))

(event `InputAction|Deflect Paper`
  (params (Key :type "Key Structure"))
  (:`Pressed`
    (set `self.DeflectPaper` true)
    (`self.AnimDeflectPaper`)
    (`KismetSystemLibrary.Delay` 2.0)
    (set `self.DeflectPaper` false))
  (:`Released`
    (set `self.DeflectPaper` false)
    (`self.AnimCharIdle`)))

(event `AnimCharIdle`
  ;[1 1 1] set 2d anim
  (bind _returnvalue (`GameplayStatics.GetActorOfClass` "/Game/_Main/Blueprints/BP_2dChar.BP_2dChar_C"))
  (`/Game/_Main/Blueprints/BP_2dChar.2dAnimCharIdle` _returnvalue))

(event `InputAction|Deflect Pouch`
  (params (Key :type "Key Structure"))
  (:`Pressed`
    (set `self.DeflectPouch` true)
    (bind _returnvalue (`GameplayStatics.GetActorOfClass` "/Game/_Main/Blueprints/BP_2dChar.BP_2dChar_C"))
    (`/Game/_Main/Blueprints/BP_2dChar.2dAnimCharDeflectPouch` _returnvalue)
    (`KismetSystemLibrary.Delay` 2.0)
    (bind _returnvalue_2 (`GameplayStatics.GetActorOfClass` "/Game/_Main/Blueprints/BP_2dChar.BP_2dChar_C"))
    (`/Game/_Main/Blueprints/BP_2dChar.2dAnimCharIdle` _returnvalue_2)
    (set `self.DeflectPouch` false))
  (:`Released`
    (set `self.DeflectPouch` false)
    (bind _returnvalue_3 (`GameplayStatics.GetActorOfClass` "/Game/_Main/Blueprints/BP_2dChar.BP_2dChar_C"))
    (`/Game/_Main/Blueprints/BP_2dChar.2dAnimCharIdle` _returnvalue_3)))

(event `self.CapsuleComponent.OnComponentBeginOverlap`
  (params (OverlappedComponent :type "PrimitiveComponent Object Reference") (OtherActor :type "Actor Object Reference") (OtherComp :type "PrimitiveComponent Object Reference") (OtherBodyIndex :type Integer) (bFromSweep :type Boolean) (SweepResult :type "HitResult Structure (by ref)"))
  (`SkeletalMeshComponent.PlayAnimation` (`self.Mesh`) "/Game/Characters/Mannequin_UE4/Animations/Jog_Fwd.Jog_Fwd" false))

(fn `UserConstructionScript`)